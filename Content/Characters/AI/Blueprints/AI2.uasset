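; AI2 is an AI character that patrols back and forth and dies when its health runs out.
; On BeginPlay it takes the mesh location as origin, then AI Move To offsets the target by MovingVector, flipping its X and Y after each successful move to loop.
; The health interface function ActorTakingDamage reduces HP and destroys the actor at zero.
; The AITakeDamages event is marked unused, and the behavior tree startup is disconnected.
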(event Custom|GetOriginPostion
  ;[1 1 1] AI Get Origin
  (Variables|Default|SetOriginPosition (Transformation|GetWorldLocation (Variables|Character|GetMesh))))

(event Custom|AI%20MoveToPos
  ;[1 1 1] AI Move To Pos
  (bind _output_get (Variables|Default|SetOriginPosition (+ (Variables|Default|GetOriginPosition) (Variables|Default|GetMovingVector))))
  (AI|AIMoveTo self _output_get 0 5.0 true
    (:OnSuccess
      (Variables|Default|SetMovingVector (* (Variables|Default|GetMovingVector) "-1.000000,-1.000000,1.000000"))
      (CallFunction|AIMovetoPos))))

(event Custom|AI%20TakeDamages
  (params (Damages :type Integer))
  ;[1 0.7823 0] AI TakeDamages (Not Used Due To Healt Interface Fct)
  (bind _output_get (Variables|Default|SetHP (- (Variables|Default|GetHP) Damages)))
  (if (<= _output_get 0)
    (CallFunction|AIDeath)))

(event Custom|AI%20Death
  ;[1 1 1] AI Death
  (Actor|DestroyActor))

(event EventBeginPlay
  ;[1 1 1] Begin Play
  (CallFunction|GetOriginPostion)
  (CallFunction|AIMovetoPos))

(fn ConstructionScript)

(fn ActorTakingDamage
  (params (Current%20Taking%20Damage :type Integer))
  (bind _output_get (Variables|Default|SetHP (- (Variables|Default|GetHP) Current%20Taking%20Damage)))
  (if (<= _output_get 0)
    (CallFunction|AIDeath)
    (return)))