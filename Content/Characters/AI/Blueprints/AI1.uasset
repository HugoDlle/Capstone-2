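; AI1 is an AI-controlled enemy that takes damage and pays the player a reward when killed.
; On BeginPlay it runs the BT_AI1 behavior tree through its AI controller, if that controller is valid.
; ActorTakingDamage subtracts damage from HP; at zero or below it fires AIDeath, which destroys the actor, then adds a fixed amount to the passed player reference's Money.
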(event Custom|AI%20Death
  ;[1 1 1] AI Death
  (Actor|DestroyActor))

(event EventBeginPlay
  (bind _self self)
  (bind _returnvalue (AI|GetAIController _self))
  ;[1 1 1] Begin Play
  ;[0.01803 1 0] Running Behavior Tree
  (Utilities|IsValid _returnvalue
    (:Is%20Valid
      (AI|RunBehaviorTree _returnvalue "/Game/Characters/AI/Behaviour/BT_AI1.BT_AI1"))))

(fn ConstructionScript)

(fn ActorTakingDamage
  (params (Current%20Taking%20Damage :type Integer) (Player%20Ref :type BP%20Player%20Object%20Reference))
  (bind _output_get (Variables|Default|SetHP (- (Variables|Default|GetHP) Current%20Taking%20Damage)))
  (if (<= _output_get 0)
    (CallFunction|AIDeath)
    (Variables|/Game/Characters/Player/ThirdPerson/Blueprints/BP_Player.BP_Player_C|SetMoney Player%20Ref (+ (Variables|/Game/Characters/Player/ThirdPerson/Blueprints/BP_Player.BP_Player_C|GetMoney Player%20Ref) 50))
    (return)))