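; BP_BoxOneShot is a map trigger box that deals massive one-shot damage to the player on contact.
; On Box overlap it casts to BP_Player and sends ActorTakingDamageMessage with a very large damage value.
; A separate looping-timer damage-over-time path lowers the player's Vie, clamped, until Compteur reaches Durée, but nothing in this graph calls its damage event.
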(event OnComponentBeginOverlap(Box)
  (params (OverlappedComponent :type Primitive%20Component%20Object%20Reference) (OtherActor :type Actor%20Object%20Reference) (OtherComp :type Primitive%20Component%20Object%20Reference) (OtherBodyIndex :type Integer) (bFromSweep :type Boolean) (SweepResult :type Hit%20Result%20Structure%20%28by%20ref%29))
  (bind _asbp_player (Utilities|Casting|CastToBP_Player OtherActor))
  (Class|HealtInterface|ActorTakingDamage(Message) _asbp_player 1000))

(event Custom|damage
  (bind _returnvalue (Utilities|Time|SetTimerbyEvent (delegate Custom|takeDamage) 1.0 true)))

(event Custom|takeDamage
  (if (< (Variables|Components|Getcompteur) (Variables|Components|Getdurée))
    (Variables|/Game/Characters/Player/ThirdPerson/Blueprints/BP_Player.BP_Player_C|SetVie (stale OnComponentBeginOverlap(Box) _asbp_player) (Math|Float|Clamp(Float) (- (Variables|/Game/Characters/Player/ThirdPerson/Blueprints/BP_Player.BP_Player_C|GetVie (stale OnComponentBeginOverlap(Box) _asbp_player)) (Variables|Components|GetpointDamage)) 0.0 (Variables|/Game/Characters/Player/ThirdPerson/Blueprints/BP_Player.BP_Player_C|GetVieMax (stale OnComponentBeginOverlap(Box) _asbp_player))))
    (Math|Integer|IncrementInt (Variables|Components|Getcompteur))
    (else
      (Utilities|Time|ClearandInvalidateTimerbyHandle (stale Custom|damage _returnvalue)))))

(fn ConstructionScript)