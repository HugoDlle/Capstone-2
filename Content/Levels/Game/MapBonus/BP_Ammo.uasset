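; BP_Ammo is an ammo bonus pickup that exists for a limited time on the map.
; When a BP_Player overlaps its Box, it calls PlayerAmmoBonus on that player and destroys itself.
; After an initial delay, a timed loop through the ResetLifetime event blinks the Ammo component's visibility as an expiry warning, then destroys the actor once a toggle counter runs out.
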(event OnComponentBeginOverlap(Box)
  (params (OverlappedComponent :type Primitive%20Component%20Object%20Reference) (OtherActor :type Actor%20Object%20Reference) (OtherComp :type Primitive%20Component%20Object%20Reference) (OtherBodyIndex :type Integer) (bFromSweep :type Boolean) (SweepResult :type Hit%20Result%20Structure%20%28by%20ref%29))
  ;[0 1 0] Bonus Ammo Logic
  (bind _asbp_player (Utilities|Casting|CastToBP_Player OtherActor))
  (Default|PlayerAmmoBonus _asbp_player)
  (Actor|DestroyActor))

(event Custom|Reset%20Lifetime
  ;[0 1 0] Bonus Display (Lifetime)
  (Utilities|FlowControl|Delay 0.5)
  (if (Variables|Default|GetIs%20visible%20?)
    (Variables|Default|SetIs%20visible%20? false)
    (Rendering|SetVisibility (Variables|Default|GetAmmo) true true)
    (else
      (Variables|Default|SetIs%20visible%20? true)
      (Rendering|SetVisibility (Variables|Default|GetAmmo) false true)))
  (Variables|Default|SetIdx (+ (Variables|Default|GetIdx) 1))
  (if (<= (Variables|Default|GetIdx) 8)
    (CallFunction|ResetLifetime)
    (else
      (Actor|DestroyActor))))

(event EventBeginPlay
  ;[0 1 0] Bonus Display (Lifetime)
  (Utilities|FlowControl|Delay 5.0)
  (if (Variables|Default|GetIs%20visible%20?)
    (Variables|Default|SetIs%20visible%20? false)
    (Rendering|SetVisibility (Variables|Default|GetAmmo) true true)
    (else
      (Variables|Default|SetIs%20visible%20? true)
      (Rendering|SetVisibility (Variables|Default|GetAmmo) false true)))
  (Variables|Default|SetIdx (+ (Variables|Default|GetIdx) 1))
  (if (<= (Variables|Default|GetIdx) 8)
    (CallFunction|ResetLifetime)
    (else
      (Actor|DestroyActor))))

(fn ConstructionScript)