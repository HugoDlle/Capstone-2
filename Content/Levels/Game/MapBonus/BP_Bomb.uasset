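; BP_Bomb is a map bonus pickup that wipes out enemy AI when the player touches it.
; A Box overlap by BP_Player calls AIDeath on every AI1 actor in the level, plays a 2D bomb sound, then destroys the bonus.
; On BeginPlay, the Bomb component blinks off and on once after a delay, but no timed destroy is connected, so the pickup stays until collected.
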(event OnComponentBeginOverlap(Box)
  (params (OverlappedComponent :type Primitive%20Component%20Object%20Reference) (OtherActor :type Actor%20Object%20Reference) (OtherComp :type Primitive%20Component%20Object%20Reference) (OtherBodyIndex :type Integer) (bFromSweep :type Boolean) (SweepResult :type Hit%20Result%20Structure%20%28by%20ref%29))
  ;[0.08127 1 0] Bonus Bomb Logic
  (Utilities|Casting|CastToBP_Player OtherActor)
  (bind _outactors (Actor|GetAllActorsOfClass "/Game/Characters/AI/Blueprints/AI1.AI1_C"))
  (for _array_element _outactors
    (Default|AIDeath _array_element))
  (Audio|PlaySound2D "/Game/Characters/Player/ThirdPerson/Sound/Bonus/bombe_-_rayan.bombe_-_rayan" 1.0 1.0 0.0 0 0)
  (Actor|DestroyActor))

(event EventBeginPlay
  ;[1 0 0] Bonus Display
  (Utilities|FlowControl|Delay 5.0)
  (Rendering|SetVisibility (Variables|Default|GetBomb) false false)
  (Utilities|FlowControl|Delay 0.8)
  (Rendering|SetVisibility (Variables|Default|GetBomb) true false)
  (Utilities|FlowControl|Delay 0.8))

(fn ConstructionScript)