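; BP_Skull is a skull bonus pickup that leaves every AI1 actor in the level on minimal health when the player collects it.
; On box overlap with BP_Player, it sets HP to 1 on all AI1 actors, plays a 2D sound and destroys itself.
; A timed sequence on BeginPlay hides and reshows the skull once; it does not loop or despawn the pickup.
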(event OnComponentBeginOverlap(Box)
  (params (OverlappedComponent :type Primitive%20Component%20Object%20Reference) (OtherActor :type Actor%20Object%20Reference) (OtherComp :type Primitive%20Component%20Object%20Reference) (OtherBodyIndex :type Integer) (bFromSweep :type Boolean) (SweepResult :type Hit%20Result%20Structure%20%28by%20ref%29))
  ;[0.2604 1 0] Bonus logic
  (Utilities|Casting|CastToBP_Player OtherActor)
  (bind _outactors (Actor|GetAllActorsOfClass "/Game/Characters/AI/Blueprints/AI1.AI1_C"))
  (for _array_element _outactors
    (Variables|/Game/Characters/AI/Blueprints/AI1.AI1_C|SetHP _array_element 1))
  (Audio|PlaySound2D "/Game/Characters/Player/ThirdPerson/Sound/Bonus/mort_inst_-_rayan.mort_inst_-_rayan" 1.0 1.0 0.0 0 0)
  (Actor|DestroyActor))

(event EventBeginPlay
  ;[1 0 0] Bonus Display
  (Utilities|FlowControl|Delay 5.0)
  (Rendering|SetVisibility (Variables|Default|GetSkull) false false)
  (Utilities|FlowControl|Delay 0.8)
  (Rendering|SetVisibility (Variables|Default|GetSkull) true false)
  (Utilities|FlowControl|Delay 0.8))

(fn ConstructionScript)