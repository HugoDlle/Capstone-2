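; Buyable player "atout" pickup granting an armor, damage, speed or money boost, with Niagara color set by type.
; Box overlap shows an item info widget and registers the pickup as the player's buyable item.
; On purchase, it refunds duplicates or adds the boost to a three-slot array, shifting out the oldest when full.
; It then resets all player multipliers, rebuilds them from that array and refreshes the player info widget.
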(event OnComponentBeginOverlap(Box)
  (params (OverlappedComponent :type Primitive%20Component%20Object%20Reference) (OtherActor :type Actor%20Object%20Reference) (OtherComp :type Primitive%20Component%20Object%20Reference) (OtherBodyIndex :type Integer) (bFromSweep :type Boolean) (SweepResult :type Hit%20Result%20Structure%20%28by%20ref%29))
  (bind _asbp_player_bis (Utilities|Casting|CastToBP_Player OtherActor))
  (Variables|Default|SetPlayer%20Ref _asbp_player_bis)
  (bind _asplayer_controller (Utilities|Casting|CastToPlayerController (Pawn|GetController _asbp_player_bis)))
  (bind _returnvalue (UserInterface|CreateWidget "/Game/Characters/Player/ThirdPerson/Widgets/HUD_ShowBuyableItem.HUD_ShowBuyableItem_C" _asplayer_controller))
  (bind _output_get (Variables|Default|SetWidget%20Ref _returnvalue))
  (UserInterface|Viewport|AddtoViewport _output_get 0)
  (Default|ShowItemInfoText _output_get (Variables|AtoutInfo|GetInfo%20Struct))
  (Variables|/Game/Characters/Player/ThirdPerson/Blueprints/BP_Player.BP_Player_C|SetCan%20Buy%20Item%20? _asbp_player_bis true)
  (Variables|/Game/Characters/Player/ThirdPerson/Blueprints/BP_Player.BP_Player_C|SetBuyable%20Item%20Ref _asbp_player_bis self))

(event OnComponentEndOverlap(Box)
  (params (OverlappedComponent :type Primitive%20Component%20Object%20Reference) (OtherActor :type Actor%20Object%20Reference) (OtherComp :type Primitive%20Component%20Object%20Reference) (OtherBodyIndex :type Integer))
  (bind _asbp_player_bis (Utilities|Casting|CastToBP_Player OtherActor))
  (Widget|RemovefromParent (Variables|Default|GetWidget%20Ref))
  (Variables|/Game/Characters/Player/ThirdPerson/Blueprints/BP_Player.BP_Player_C|SetCan%20Buy%20Item%20? _asbp_player_bis false))

(event EventBeginPlay
  (switch Utilities|FlowControl|Switch|SwitchonE_PlayerAtout (Variables|AtoutInfo|GetE_PlayerAtout)
    (:NewEnumerator0
      (Class|NiagaraComponent|SetAsset (Variables|Default|GetNiagara) "/Game/Levels/Game/PlayerAtout/Green_Mat/Green_AtoutParticuleSysteme.Green_AtoutParticuleSysteme" true))
    (:NewEnumerator1
      (Class|NiagaraComponent|SetAsset (Variables|Default|GetNiagara) "/Game/Levels/Game/PlayerAtout/Red_Mat/Red_AtoutParticuleSysteme.Red_AtoutParticuleSysteme" true))
    (:NewEnumerator2
      (Class|NiagaraComponent|SetAsset (Variables|Default|GetNiagara) "/Game/Levels/Game/PlayerAtout/Blue_Mat/Blue_AtoutParticuleSysteme1.Blue_AtoutParticuleSysteme1" true))
    (:NewEnumerator3
      (Class|NiagaraComponent|SetAsset (Variables|Default|GetNiagara) "/Game/Levels/Game/PlayerAtout/Yellow_Mat/Yellow_AtoutParticuleSysteme1.Yellow_AtoutParticuleSysteme1" true))))

(event EventItemIsBuy
  (bind _player_ref (Variables|Default|GetPlayer%20Ref))
  ;[0.01467 1 0] Item Is Buy Logic
  (Utilities|FlowControl|Sequence
    (:then_0
      (if (< (Utilities|Array|Length (Variables|/Game/Characters/Player/ThirdPerson/Blueprints/BP_Player.BP_Player_C|GetPlayer%20Array%20Atout (Variables|Default|GetPlayer%20Ref))) 3)
        (if (|IsPlayerHasn'tItem?)
          (Utilities|Array|Add (Variables|/Game/Characters/Player/ThirdPerson/Blueprints/BP_Player.BP_Player_C|GetPlayer%20Array%20Atout (Variables|Default|GetPlayer%20Ref)) (Variables|AtoutInfo|GetE_PlayerAtout))
          (|WichAtoutStats)
          (else
            (Variables|/Game/Characters/Player/ThirdPerson/Blueprints/BP_Player.BP_Player_C|SetMoney _player_ref (+ (Variables|/Game/Characters/Player/ThirdPerson/Blueprints/BP_Player.BP_Player_C|GetMoney _player_ref) (.neededmoney (Variables|AtoutInfo|GetInfo%20Struct))))))
        (else
          (|AtoutRotationInPlayerArrayIfFull))))
    (:then_1
      (|SetAtoutFactorToPlayer))))

(fn ConstructionScript)

(fn GetInfoStruct
  (return (Variables|AtoutInfo|GetInfo%20Struct)))