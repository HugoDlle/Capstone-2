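; Game mode that runs an endless zombie wave survival loop and relays wave and ammo updates to all players.
; After a startup delay it caches spawners and zones, then sets the per-wave enemy increase from player count.
; Each wave activates zone spawners and queues enemies on randomly picked active spawners, retrying inactive picks.
; A looping timer detects zero remaining enemies, pauses, then launches a larger wave.
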(event Custom|CheckWaveEnd
  (if (and (== (Variables|Default|GetEnemyRemaining) 0) (== (Variables|Default|GetisWaveEnd) false))
    (Variables|Default|SetisWaveEnd true)
    (Utilities|FlowControl|Delay 1e+01)
    (Variables|Default|SetEnemyMaxCount (+ (Variables|Default|GetEnemyMaxCount) (Variables|Default|GetZombieIncrement)))
    (CallFunction|NewWave)))

(event Custom|New%20Wave
  ;[1 1 1] New Wave
  (Variables|Default|SetisWaveEnd false)
  (Math|Integer|IncrementInt (Variables|Default|GetWaveNumber)
    (:%20%20
      (CallFunction|Test)
      (for _array_element (Variables|Default|GetSpawnZones)
        (Default|ActivateSpawners _array_element))
      (CallFunction|StartWave))))

(event Custom|Player%20Update%20Max%20Ammo
  ;[1 1 1] testy
  (bind _outactors (Actor|GetAllActorsOfClass "/Game/Characters/Player/ThirdPerson/Blueprints/BP_Player.BP_Player_C"))
  (for _array_element _outactors
    (Default|PlayerRefreshAmmo _array_element)))

(event Custom|Test
  ;[1 1 1] testy
  (bind _outactors (Actor|GetAllActorsOfClass "/Game/Characters/Player/ThirdPerson/Blueprints/BP_Player.BP_Player_C"))
  (for _array_element _outactors
    (Default|PlayerUpdateWave _array_element (Variables|Default|GetWaveNumber))))

(event EventBeginPlay
  (Utilities|FlowControl|Delay 3e+01)
  (CallFunction|GetSpawners)
  (CallFunction|GetNumberOfPlayers)
  (CallFunction|NewWave)
  (Utilities|Time|SetTimerbyEvent (delegate Custom|CheckWaveEnd) 2.0 true 1e+01))

(event EventPostLogin
  (params (NewPlayer :type Player%20Controller%20Object%20Reference))
  (switch int (Math|Random|RandomIntegerinRange 0 3)))

(fn ConstructionScript)

(fn GetSpawners
  (bind _outactors (Actor|GetAllActorsOfClass "/Game/Characters/AI/Spawner/AI_Spawner.AI_Spawner_C"))
  (Variables|Default|SetSpawners _outactors)
  (bind _outactors_2 (Actor|GetAllActorsOfClass "/Game/Characters/AI/Spawner/SpawnZone.SpawnZone_C"))
  (Variables|Default|SetSpawnZones _outactors_2))

(fn StartWave
  (for _index (range 1 (Variables|Default|GetEnemyMaxCount))
    (bind _output_get (LocalVariables|SetValidSpawner (.OutItem (Utilities|Array|Random (Variables|Default|GetSpawners))) :!label _label))
    (if (Variables|/Game/Characters/AI/Spawner/AI_Spawner.AI_Spawner_C|GetisActivated _output_get)
      (Default|AddEnemytoQueue (LocalVariables|GetValidSpawner))
      (else
        (goto _label)))))

(fn GetNumberOfPlayers
  (bind _outactors (Actor|GetAllActorsOfClass "/Game/Characters/Player/ThirdPerson/Blueprints/BP_Player.BP_Player_C"))
  (Variables|Default|SetZombieIncrement (* (Utilities|Array|Length _outactors) 2)))