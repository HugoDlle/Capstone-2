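; BP_BuyableRuinsDoor is a purchasable door that disappears once bought.
; Its Box overlap shows a HUD_ShowBuyableItem widget with InfoStruct and registers the door on BP_Player as buyable, until exit.
; ItemIsBuy marks it bought and, if the widget is valid, removes it, moves the mesh over time, then destroys the actor.
; The move target comes from MouvementCalculToSendToServer, whose height-based drop calculation is left unconnected.
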(event OnComponentBeginOverlap(Box)
  (params (OverlappedComponent :type Primitive%20Component%20Object%20Reference) (OtherActor :type Actor%20Object%20Reference) (OtherComp :type Primitive%20Component%20Object%20Reference) (OtherBodyIndex :type Integer) (bFromSweep :type Boolean) (SweepResult :type Hit%20Result%20Structure%20%28by%20ref%29))
  ;[0.06385 1 0] Display/Not display item info to player logic
  (bind _asbp_player (Utilities|Casting|CastToBP_Player OtherActor))
  (if (not (Variables|Default|GetIs%20Buy%20?))
    (Variables|Default|SetPlayer%20Ref _asbp_player)
    (bind _asplayer_controller (Utilities|Casting|CastToPlayerController (Pawn|GetController _asbp_player)))
    (bind _returnvalue (UserInterface|CreateWidget "/Game/Characters/Player/ThirdPerson/Widgets/HUD_ShowBuyableItem.HUD_ShowBuyableItem_C" _asplayer_controller))
    (bind _output_get (Variables|Default|SetWidget%20Ref _returnvalue))
    (UserInterface|Viewport|AddtoViewport _output_get 0)
    (Default|ShowItemInfoText _output_get (Variables|Default|GetInfo%20Struct))
    (Variables|/Game/Characters/Player/ThirdPerson/Blueprints/BP_Player.BP_Player_C|SetCan%20Buy%20Item%20? _asbp_player true)
    (Variables|/Game/Characters/Player/ThirdPerson/Blueprints/BP_Player.BP_Player_C|SetBuyable%20Item%20Ref _asbp_player self)))

(event OnComponentEndOverlap(Box)
  (params (OverlappedComponent :type Primitive%20Component%20Object%20Reference) (OtherActor :type Actor%20Object%20Reference) (OtherComp :type Primitive%20Component%20Object%20Reference) (OtherBodyIndex :type Integer))
  ;[0.06385 1 0] Display/Not display item info to player logic
  (bind _asbp_player (Utilities|Casting|CastToBP_Player OtherActor))
  (if (not (Variables|Default|GetIs%20Buy%20?))
    (Widget|RemovefromParent (Variables|Default|GetWidget%20Ref))
    (Variables|/Game/Characters/Player/ThirdPerson/Blueprints/BP_Player.BP_Player_C|SetCan%20Buy%20Item%20? _asbp_player false)))

(event EventItemIsBuy
  (bind (_point_after_deplacement _point_after_deplacement_x _point_after_deplacement_y _point_after_deplacement_z _item_rot) (|MouvementCalculToSendToServer))
  ;[0.06385 1 0] Item Logic After Buy
  (Variables|/Game/Characters/Player/ThirdPerson/Blueprints/BP_Player.BP_Player_C|SetCan%20Buy%20Item%20? (Variables|Default|GetPlayer%20Ref) false)
  (Variables|Default|SetIs%20Buy%20? true)
  (Utilities|IsValid (Variables|Default|GetWidget%20Ref)
    (:Is%20Valid
      (Widget|RemovefromParent (Variables|Default|GetWidget%20Ref))
      (Components|MoveComponentTo (Variables|Default|GetStaticMeshComponent0) (Math|Vector|MakeVector _point_after_deplacement_x _point_after_deplacement_y _point_after_deplacement_z) _item_rot false true 1.5 false)
      (Actor|DestroyActor))))

(fn ConstructionScript)

(fn GetInfoStruct
  (return (Variables|Default|GetInfo%20Struct)))