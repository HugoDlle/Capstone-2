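; Purchasable door that swings open when bought, then closes and becomes buyable again after a short delay.
; Its box overlap shows a price widget and registers the door on the player as the current buyable item.
; ItemIsBuy removes the widget, routes mesh rotation through the player's PlayerMoveDoor, and starts the reset timer.
; An info-struct setter, apparently invoked as an interface message on purchase, raises the cost each time.
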(event OnComponentBeginOverlap(Box)
  (params (OverlappedComponent :type Primitive%20Component%20Object%20Reference) (OtherActor :type Actor%20Object%20Reference) (OtherComp :type Primitive%20Component%20Object%20Reference) (OtherBodyIndex :type Integer) (bFromSweep :type Boolean) (SweepResult :type Hit%20Result%20Structure%20%28by%20ref%29))
  ;[0 1 0] Display/Not display item info to player logic
  (bind _asbp_player_bis (Utilities|Casting|CastToBP_Player OtherActor))
  (if (not (Variables|Default|GetIs%20Buy%20?))
    (Variables|Default|SetPlayer%20ref _asbp_player_bis)
    (bind _asplayer_controller (Utilities|Casting|CastToPlayerController (Pawn|GetController _asbp_player_bis)))
    (bind _returnvalue (UserInterface|CreateWidget "/Game/Characters/Player/ThirdPerson/Widgets/HUD_ShowBuyableItem.HUD_ShowBuyableItem_C" _asplayer_controller))
    (bind _output_get (Variables|Default|SetWidget%20Ref _returnvalue))
    (UserInterface|Viewport|AddtoViewport _output_get 0)
    (Default|ShowItemInfoText _output_get (Variables|Default|GetInfo%20Struct))
    (Variables|/Game/Characters/Player/ThirdPerson/Blueprints/BP_Player.BP_Player_C|SetCan%20Buy%20Item%20? _asbp_player_bis true)
    (Variables|/Game/Characters/Player/ThirdPerson/Blueprints/BP_Player.BP_Player_C|SetBuyable%20Item%20Ref _asbp_player_bis self)))

(event OnComponentEndOverlap(Box)
  (params (OverlappedComponent :type Primitive%20Component%20Object%20Reference) (OtherActor :type Actor%20Object%20Reference) (OtherComp :type Primitive%20Component%20Object%20Reference) (OtherBodyIndex :type Integer))
  ;[0 1 0] Display/Not display item info to player logic
  (bind _asbp_player_bis (Utilities|Casting|CastToBP_Player OtherActor))
  (if (not (Variables|Default|GetIs%20Buy%20?))
    (Widget|RemovefromParent (Variables|Default|GetWidget%20Ref))
    (Variables|/Game/Characters/Player/ThirdPerson/Blueprints/BP_Player.BP_Player_C|SetCan%20Buy%20Item%20? _asbp_player_bis false)))

(event Custom|Open%20Door%20Timer
  (bind _staticmesh (Variables|Default|GetStaticMesh))
  (bind _returnvalue (Transformation|GetWorldRotation _staticmesh))
  (Utilities|FlowControl|Delay 5.0)
  (Variables|Default|SetIs%20Buy%20? false)
  (Default|PlayerMoveDoor (Variables|Default|GetPlayer%20ref) _staticmesh (Transformation|GetWorldLocation _staticmesh) (Math|Rotator|MakeRotator (+ (.roll _returnvalue) 6e+01) (.pitch _returnvalue) (.yaw _returnvalue))))

(event EventItemIsBuy
  (bind _staticmesh (Variables|Default|GetStaticMesh))
  (bind _returnvalue (Transformation|GetWorldRotation _staticmesh))
  ;[0 1 0] item is buy
  (Variables|/Game/Characters/Player/ThirdPerson/Blueprints/BP_Player.BP_Player_C|SetCan%20Buy%20Item%20? (Variables|Default|GetPlayer%20Ref) false)
  (Utilities|IsValid (Variables|Default|GetWidget%20Ref)
    (:Is%20Valid
      (Widget|RemovefromParent (Variables|Default|GetWidget%20Ref))
      (Variables|Default|SetIs%20Buy%20? true)
      (Default|PlayerMoveDoor (Variables|Default|GetPlayer%20ref) _staticmesh (Transformation|GetWorldLocation _staticmesh) (Math|Rotator|MakeRotator (+ (.roll _returnvalue) -6e+01) (.pitch _returnvalue) (.yaw _returnvalue)))
      (Class|BuyableItemInterface|SetInfoStruct(Message) self)
      (CallFunction|OpenDoorTimer))))

(event EventSetInfoStruct
  (Variables|Default|SetInfo%20Struct (Utilities|Struct|MakeBuyableStructureObject (+ (.neededmoney (Variables|Default|GetInfo%20Struct)) 500) (.objectname (Variables|Default|GetInfo%20Struct)))))

(fn ConstructionScript)

(fn OnRepIsBuy?)

(fn GetInfoStruct
  (return (Variables|Default|GetInfo%20Struct)))